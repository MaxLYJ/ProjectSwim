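; BP_FieldImpact is a Chaos field system test Blueprint that breaks and pushes destructible objects on impact.
; When its Sphere begins overlapping a BP_LockOnTarget, it stores that target and sets an overlap flag.
; It applies a sphere-sized external cluster strain field without falloff, then a strong radial linear force centred on the world origin rather than the sphere.
; An unconnected variant with weaker strain and sphere-centred force never runs.
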(event OnComponentBeginOverlap(Sphere)
  (params (OverlappedComponent :type Primitive%20Component%20Object%20Reference) (OtherActor :type Actor%20Object%20Reference) (OtherComp :type Primitive%20Component%20Object%20Reference) (OtherBodyIndex :type Integer) (bFromSweep :type Boolean) (SweepResult :type Hit%20Result%20Structure%20%28by%20ref%29))
  (bind _fieldsystemcomponent (Variables|Field|GetFieldSystemComponent))
  (bind _sphere (Variables|Default|GetSphere))
  ;[1 1 1] Break the object
  (bind _asbp_lock_on_target (Utilities|Casting|CastToBP_LockOnTarget OtherActor))
  (Variables|Default|SetAs%20BP%20Lock%20On%20Target _asbp_lock_on_target)
  (Class|FieldSystemComponent|ApplyPhysicsField _fieldsystemcomponent true "Field_ExternalClusterStrain" 0 (Field|SetRadialFalloff (Variables|Default|GetRadialFalloff) 1e+06 0.0 1.0 0.0 (Variables|/Script/Engine.SphereComponent|GetSphereRadius _sphere) (Transformation|GetWorldLocation _sphere) "Field_FallOff_None"))
  (Variables|Default|SetIsOverlap true)
  (Class|FieldSystemComponent|ApplyPhysicsField _fieldsystemcomponent true "Field_LinearForce" 0 (Field|SetRadialVector (Variables|Default|GetRadialVector) 1.2e+07 "0, 0, 0")))

(event EventTick
  (params (DeltaSeconds :type Float%20%28single-precision%29)))

(event EventBeginPlay
  ;[1 1 1] Debug testing chaos system
)

(fn ConstructionScript)