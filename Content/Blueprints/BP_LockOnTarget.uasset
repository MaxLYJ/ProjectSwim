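; BP_LockOnTarget is a lock-on target actor that glows and releases the player's lock when hit by a charge.
; BeginPlay creates a dynamic highlight material on its sphere geometry collection.
; Tick drives that material's highlight intensity from the target's LockOnEmissive plus the first-person character's sonar progression.
; When a charging first-person character overlaps Sphere1, the character's IsLockTarget flag is cleared.
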(event OnComponentBeginOverlap(Sphere1)
  (params (OverlappedComponent :type Primitive%20Component%20Object%20Reference) (OtherActor :type Actor%20Object%20Reference) (OtherComp :type Primitive%20Component%20Object%20Reference) (OtherBodyIndex :type Integer) (bFromSweep :type Boolean) (SweepResult :type Hit%20Result%20Structure%20%28by%20ref%29))
  ;[1 1 1] Remove lock after hit by the player character
  (bind _asbp_first_person_character (Utilities|Casting|CastToBP_FirstPersonCharacter OtherActor))
  (if (Variables|/Game/FirstPerson/Blueprints/BP_FirstPersonCharacter.BP_FirstPersonCharacter_C|GetIsCharging _asbp_first_person_character)
    (Variables|/Game/FirstPerson/Blueprints/BP_FirstPersonCharacter.BP_FirstPersonCharacter_C|SetIsLockTarget _asbp_first_person_character false)))

(event EventBeginPlay
  ;[1 1 1] Initialization
  (bind _returnvalue (Rendering|Material|CreateDynamicMaterialInstance (Variables|Default|GetSphere_GeometryCollection) 0 "/Game/FirstPerson/Materials/M_Highlight_Inst.M_Highlight_Inst" "None" :!class /Script/Engine.PrimitiveComponent))
  (Variables|Default|SetM_Highlight2 _returnvalue))

(event EventTick
  (params (DeltaSeconds :type Float%20%28single-precision%29))
  ;[1 1 1] Set object emissive on lock
  (Utilities|FlowControl|Sequence
    (:then_0
      (bind _asbp_first_person_character (Utilities|Casting|CastToBP_FirstPersonCharacter (Game|GetPlayerCharacter 0)))
      (Rendering|Material|SetScalarParameterValue (Variables|Default|GetM_Highlight2) "HightLightIntensity" (+ (* (Variables|Default|GetLockOnEmissive) 5.0) (* (Variables|/Game/FirstPerson/Blueprints/BP_FirstPersonCharacter.BP_FirstPersonCharacter_C|GetSonarProcression _asbp_first_person_character) 5.0)) :!class /Script/Engine.MaterialInstanceDynamic))))

(fn ConstructionScript)